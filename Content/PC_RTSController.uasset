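; RTS player controller that handles mouse input setup and camera zoom.
; On BeginPlay it sets Game and UI input mode with the mouse locked to the viewport and caches its view target as a BP_RTSCamera.
; The mouse wheel axis adjusts a clamped zoom factor, which maps linearly to the camera's spring arm length.
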(event EventBeginPlay
  (Input|SetInputModeGameandUI self 0 "LockAlways" false)
  (bind _asbp_rtscamera (Utilities|Casting|CastToBP_RTSCamera (Pawn|GetViewTarget)))
  (Variables|Default|SetAs%20BP%20RTSCamera _asbp_rtscamera))

(event Input|MouseEvents|MouseWheelAxis
  (params (AxisValue :type Float%20%28single-precision%29))
  (bind _output_get (Variables|Default|SetZoomFactor (Math|Float|Clamp(Float) (+ (Variables|Default|GetZoomFactor) (* AxisValue -1.0)) 0.0 1e+01)))
  (Variables|/Script/Engine.SpringArmComponent|SetTargetArmLength (Variables|/Game/BP_RTSCamera.BP_RTSCamera_C|GetSpringArm (Variables|Default|GetAs%20BP%20RTSCamera)) (+ (* _output_get 2e+02) 1e+03)))

(fn ConstructionScript)