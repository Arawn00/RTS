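; RTS HUD Blueprint that draws a translucent cyan drag-selection box on screen; it does not select any actors itself.
; StartSelection stores the viewport-scaled mouse position as the anchor corner and enables drawing, while StopSelection disables it.
; While drawing is enabled, each DrawHUD call samples the mouse again and draws a canvas rectangle from the anchor using signed width and height.
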(event EventStartSelection
  (bind _returnvalue (Class|WidgetLayoutLibrary|GetMousePositiononViewport))
  (Variables|Default|SetPointA (Math|Vector2D|MakeVector2D (.x (* _returnvalue (Class|WidgetLayoutLibrary|GetViewportScale))) (.y (* _returnvalue (Class|WidgetLayoutLibrary|GetViewportScale)))))
  (Variables|Default|SetIsDrawing true))

(event EventStopSelection
  (Variables|Default|SetIsDrawing false))

(event EventDrawHUD
  (params (SizeX :type Integer) (SizeY :type Integer))
  (bind _pointa (Variables|Default|GetPointA))
  ;[1 1 1] Draw Rect
  (if (Variables|Default|GetIsDrawing)
    (bind _returnvalue (Class|WidgetLayoutLibrary|GetMousePositiononViewport))
    (Variables|Default|SetPointB (Math|Vector2D|MakeVector2D (.x (* _returnvalue (Class|WidgetLayoutLibrary|GetViewportScale))) (.y (* _returnvalue (Class|WidgetLayoutLibrary|GetViewportScale)))))
    (HUD|DrawRect "(R=0.000000,G=0.856858,B=0.937500,A=0.500000)" (.x _pointa) (.y _pointa) (- (.x (Variables|Default|GetPointB)) (.x _pointa)) (- (.y (Variables|Default|GetPointB)) (.y _pointa)))))

(fn ConstructionScript)