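; Behavior tree task that sends a unit to the capital building to deposit the wood it carries.
; It finds a Bp_BuildingCapital actor and uses AIMoveTo to walk the pawn there.
; On arrival it adds the carried wood to the RTSGameMode inventory, clears the unit's load, refreshes its frame and finishes successfully.
; A missing capital or failed move never calls FinishExecute.
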(event EventReceiveExecuteAI
  (params (OwnerController :type AI%20Controller%20Object%20Reference) (ControlledPawn :type Pawn%20Object%20Reference))
  (bind _asbp_unit_base (Utilities|Casting|CastTobp_UnitBase ControlledPawn))
  (Variables|Default|SetAs%20Bp%20Unit%20Base _asbp_unit_base)
  (bind _returnvalue (Actor|GetActorOfClass "/Game/Blueprints/Buildings/bp_BuildingCapital.bp_BuildingCapital_C"))
  (Utilities|IsValid _returnvalue
    (:Is%20Valid
      (AI|AIMoveTo ControlledPawn "0, 0, 0" _returnvalue 5.0 false
        (:OnSuccess
          (bind _asrtsgame_mode (Utilities|Casting|CastToRTSGameMode (Game|GetGameMode)))
          (Variables|/Game/Blueprints/RTSGameMode.RTSGameMode_C|SetWoodInventory _asrtsgame_mode (+ (Variables|/Game/Blueprints/RTSGameMode.RTSGameMode_C|GetWoodInventory _asrtsgame_mode) (Variables|/Game/Blueprints/Units/bp_UnitBase.bp_UnitBase_C|GetWoodCarrying (Variables|Default|GetAs%20Bp%20Unit%20Base))))
          (Variables|/Game/Blueprints/Units/bp_UnitBase.bp_UnitBase_C|SetWoodCarrying (Variables|Default|GetAs%20Bp%20Unit%20Base) 0)
          (Default|UpdateUnitFrame (Variables|Default|GetAs%20Bp%20Unit%20Base))
          (AI|BehaviorTree|FinishExecute true))))))