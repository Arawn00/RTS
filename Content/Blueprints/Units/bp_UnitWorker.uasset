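; bp_UnitWorker is a worker unit Blueprint that shows the resource it carries on its unit frame widget.
; On BeginPlay it runs the parent logic, then casts the inherited unit frame widget to w_WorkerUnitFrame and stores the reference.
; Its UpdateUnitFrame override calls the parent, repeats that cast, and passes the carried amount and held resource type to the widget's UpdateFrame.
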(event EventBeginPlay
  (|CallParentFunction)
  (bind _asw_worker_unit_frame (Utilities|Casting|CastTow_WorkerUnitFrame (Variables|Default|GetUnitFrameWidget)))
  (Variables|Default|SetAs%20W%20Worker%20Unit%20Frame _asw_worker_unit_frame))

(event Collision|EventActorBeginOverlap
  (params (OtherActor :type Actor%20Object%20Reference)))

(event EventTick
  (params (DeltaSeconds :type Float%20%28single-precision%29)))

(fn ConstructionScript
  (|CallParentFunction))

(fn UpdateUnitFrame
  (|CallParentFunction)
  (bind _asw_worker_unit_frame (Utilities|Casting|CastTow_WorkerUnitFrame (Variables|Default|GetUnitFrameWidget)))
  (Default|UpdateFrame _asw_worker_unit_frame (Variables|Default|GetRessourceCarrying) (Variables|Default|GetRessourceHeld)))