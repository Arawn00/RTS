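; Behavior tree task that makes a bp_UnitBase unit harvest the resource actor stored as its blackboard attack target.
; On execute it caches the unit, target and resource type from the pawn and blackboard.
; Each tick it slightly damages the target, increments the unit's carried amount, sets the held type and refreshes the unit frame, with no capacity check.
; Once the target is invalid, it resets the Action key and finishes successfully.
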(event EventReceiveExecuteAI
  (params (OwnerController :type AI%20Controller%20Object%20Reference) (ControlledPawn :type Pawn%20Object%20Reference))
  (bind _asbp_unit_base (Utilities|Casting|CastTobp_UnitBase ControlledPawn))
  (Variables|Default|SetAs%20Bp%20Unit%20Base _asbp_unit_base)
  (Variables|Default|SetAttackTargetRef (AI|BehaviorTree|GetBlackboardValueasActor (Variables|Default|GetAttackTarget)))
  (Variables|Default|SetRessourceRef (Utilities|Enum|ByteToEnumenum_Ressources (Class|BTFunctionLibrary|GetBlackboardValueasEnum (Variables|Default|GetRessource)))))

(event EventReceiveTickAI
  (params (OwnerController :type AI%20Controller%20Object%20Reference) (ControlledPawn :type Pawn%20Object%20Reference) (DeltaSeconds :type Float%20%28single-precision%29))
  (bind _as_bp_unit_base (Variables|Default|GetAs%20Bp%20Unit%20Base))
  (bind _attacktargetref (Variables|Default|GetAttackTargetRef))
  (Utilities|IsValid _attacktargetref
    (:Is%20Valid
      (Game|Damage|ApplyDamage _attacktargetref 0.1 0 0)
      (Variables|/Game/Blueprints/Units/bp_UnitBase.bp_UnitBase_C|SetRessourceCarrying _as_bp_unit_base (+ (Variables|/Game/Blueprints/Units/bp_UnitBase.bp_UnitBase_C|GetRessourceCarrying _as_bp_unit_base) 1))
      (Variables|/Game/Blueprints/Units/bp_UnitBase.bp_UnitBase_C|SetRessourceHeld (Variables|Default|GetAs%20Bp%20Unit%20Base) (Variables|Default|GetRessourceRef))
      (Default|UpdateUnitFrame (Variables|Default|GetAs%20Bp%20Unit%20Base)))
    (:Is%20Not%20Valid
      (Class|BTFunctionLibrary|SetBlackboardValueasEnum (Variables|Default|GetAction))
      (AI|BehaviorTree|FinishExecute true))))