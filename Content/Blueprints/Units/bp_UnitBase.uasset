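; Base unit Blueprint for an RTS that can be clicked to toggle its selection.
; A left click asks the RTS player controller to add or remove the unit, using the decal's visibility as the current selection state.
; An IsSelected event shows or hides that decal to mark the unit as selected.
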(event Custom|IsSelected
  (params (IsSelected :type Boolean))
  (Rendering|SetVisibility (Variables|Default|GetDecal) IsSelected false))

(event EventBeginPlay
  (bind _aspc_rtscontroller (Utilities|Casting|CastToPC_RTSController (Game|GetPlayerController 0)))
  (Variables|Default|SetAs%20PC%20RTSController _aspc_rtscontroller))

(event MouseInput|EventActorOnClicked
  (params (ButtonPressed :type Key%20Structure :default "None"))
  (bind _self self)
  (if (== ButtonPressed "LeftMouseButton")
    (bind _aspc_rtscontroller (Utilities|Casting|CastToPC_RTSController (Game|GetPlayerController 0)))
    (if (Rendering|IsVisible (Variables|Default|GetDecal))
      (Default|RemoveUnittoSelection _aspc_rtscontroller _self)
      (else
        (Default|AddUnittoSelection _aspc_rtscontroller _self)))))

(fn ConstructionScript)