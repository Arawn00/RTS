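; Base Blueprint for selectable RTS buildings that opens a base menu when left-clicked.
; The click clears the player controller's unit selection, runs the parent click logic, moves the camera to the building, shows the menu widget and disables zoom.
; Deselection runs the parent handler and removes the menu, but does not re-enable zoom here.
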(event EventIsSelected
  (params (IsSelected :type Boolean))
  (|CallParentFunction IsSelected)
  (if (not IsSelected)
    (Widget|RemovefromParent (Variables|Default|GetBaseMenu))
    (Variables|Default|SetBaseMenu 0)))

(event MouseInput|EventActorOnClicked
  (params (ButtonPressed :type Key%20Structure :default "None"))
  (bind _as_pc_rtscontroller (Variables|Default|GetAs%20PC%20RTSController))
  (if (== ButtonPressed "LeftMouseButton")
    (bind _aspc_rtscontroller (Utilities|Casting|CastToPC_RTSController (Game|GetPlayerController 0)))
    (Default|ClearUnitSelection _aspc_rtscontroller)
    (|CallParentFunction ButtonPressed)
    (Default|SetCameraLocation _as_pc_rtscontroller (Transformation|GetActorLocation))
    (bind _returnvalue (UserInterface|CreateWidget "/Game/UI/BaseBuildingUI/W_BaseMenui.W_BaseMenui_C"))
    (bind _output_get (Variables|Default|SetBaseMenu _returnvalue))
    (UserInterface|Viewport|AddtoViewport _output_get 0)
    (Variables|/Game/Blueprints/PC_RTSController.PC_RTSController_C|SetIsZoomEnabled _as_pc_rtscontroller false)))

(fn ConstructionScript
  (|CallParentFunction))